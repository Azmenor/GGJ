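; BP_Gear_Covoyeur is a conveyor gear that spins its static mesh and passes the motion on to a linked gear.
; On BeginPlay it calls Rotate with its own AngleDirection, which stores the direction and recursively calls Rotate on a valid GearCovoyeur reference with the sign flipped, so chained gears counter-rotate.
; A Rotation timeline then drives the mesh's relative pitch, scaled by that direction.
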(event Custom|Rotate
  (params (Angle%20Direction :type Integer))
  (bind _output_get (Variables|Default|SetAngle%20Direction Angle%20Direction))
  (bind _gear_covoyeur (Variables|Default|GetGear_Covoyeur)
    (:then
      (CallFunction|Rotate _gear_covoyeur (* _output_get -1))
      (bind _rotation (Timeline|Rotation Play)
        (:Update
          (Transformation|SetRelativeRotation (Variables|Default|GetStaticMesh) (Math|Rotator|MakeRotator 0.0 (* (Variables|Default|GetAngle%20Direction) _rotation) 0.0) false false))))
    (:else
      (Timeline|Rotation Play))))

(event EventBeginPlay
  (CallFunction|Rotate (Variables|Default|GetAngle%20Direction)))

(fn ConstructionScript)