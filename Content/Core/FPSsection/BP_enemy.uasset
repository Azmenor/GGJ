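; BP_enemy is an FPS enemy that follows a spline path and shoots at the player once BP_Player overlaps its Collision component.
; The first overlap starts a timeline scaled by spline length, while a looping timer fires BP_bullet toward the player with a sound.
; Tick feeds the player's location coordinates into the enemy's rotation and prints it as debug.
; Damage reduces PV, destroying the enemy at zero or below.
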(event OnComponentBeginOverlap(Collision)
  (params (OverlappedComponent :type Primitive%20Component%20Object%20Reference) (OtherActor :type Actor%20Object%20Reference) (OtherComp :type Primitive%20Component%20Object%20Reference) (OtherBodyIndex :type Integer) (bFromSweep :type Boolean) (SweepResult :type Hit%20Result%20Structure%20%28by%20ref%29))
  (bind _spline (Variables|Default|GetSpline))
  (bind _splinem (Variables|/Game/Core/FPSsection/BP_EnemySpline.BP_EnemySpline_C|GetSplineM _spline))
  (bind _returnvalue (Spline|GetSplineLength _splinem))
  (Utilities|Casting|CastToBP_Player OtherActor)
  (Utilities|FlowControl|Sequence
    (:then_0
      (Utilities|FlowControl|DoOnce false
        (:Completed
          (Components|Timeline|SetPlayRate (Variables|Default|GetTimeline_0) (/ 1e+03 _returnvalue))
          (bind _position (Timeline|Timeline_0 PlayFromStart)
            (:Update
              (Transformation|SetActorTransform self (Math|Transform|MakeTransform (.location (Spline|GetTransformatDistanceAlongSpline _splinem (* _position _returnvalue) "World" false)) (.rotation (Spline|GetTransformatDistanceAlongSpline _splinem (* _position _returnvalue) "World" false)) (.scale (Spline|GetTransformatDistanceAlongSpline _splinem (* _position _returnvalue) "World" false)))))))))
    (:then_1
      (Utilities|IsValid self
        (:Is%20Valid
          (Utilities|Time|SetTimerbyEvent (delegate Custom|shooting) 2.0 true))))))

(event Custom|shooting
  (Game|SpawnActorfromClass "/Game/Core/FPSsection/BP_bullet.BP_bullet_C" (Math|Transform|MakeTransform (Transformation|GetActorLocation) (Math|Rotator|FindLookatRotation (Transformation|GetWorldLocation (Variables|Default|GetSphere)) (Transformation|GetActorLocation (Game|GetPlayerCharacter 0))) "1,1,1") "Undefined" 0 self 0)
  (Audio|PlaySound2D "/Game/Core/Audio/ennemy_shots_8.ennemy_shots_8" 1.0 1.0 0.0 0 0))

(event Game|Damage|EventAnyDamage
  (params (Damage :type Float%20%28single-precision%29) (DamageType :type Damage%20Type%20Object%20Reference) (InstigatedBy :type Controller%20Object%20Reference) (DamageCauser :type Actor%20Object%20Reference))
  (bind _output_get (Variables|Default|SetPV (- (Variables|Default|GetPV) Damage)))
  (if (<= _output_get 0.0)
    (Actor|DestroyActor)))

(event EventTick
  (params (DeltaSeconds :type Float%20%28single-precision%29))
  (bind _returnvalue (Game|GetPlayerCharacter 0))
  (bind _rootcomponent (Variables|/Script/Engine.Actor|GetRootComponent _returnvalue))
  (bind _returnvalue_2 (Transformation|GetWorldLocation _rootcomponent))
  (Transformation|SetActorRotation (Math|Rotator|MakeRotator (.x _returnvalue_2) (.y _returnvalue_2) (.z _returnvalue_2)))
  (Development|PrintString (Utilities|String|ToString(Rotator) (Transformation|GetActorRotation)) true true "(R=0.000000,G=0.660000,B=1.000000,A=1.000000)" 0.0))

(fn ConstructionScript)