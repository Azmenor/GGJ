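; BP_EnemyWall is a damageable wall actor in the FPS section, built around a Cube component.
; Any damage it takes is subtracted from Health, and once that reaches zero or below the still-valid Cube component is destroyed, leaving the actor itself in place.
; An overlap between the Cube and BP_Player only prints a debug "Hello" message.
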(event OnComponentBeginOverlap(Cube)
  (params (OverlappedComponent :type Primitive%20Component%20Object%20Reference) (OtherActor :type Actor%20Object%20Reference) (OtherComp :type Primitive%20Component%20Object%20Reference) (OtherBodyIndex :type Integer) (bFromSweep :type Boolean) (SweepResult :type Hit%20Result%20Structure%20%28by%20ref%29))
  (Utilities|Casting|CastToBP_Player OtherActor)
  (Development|PrintString "Hello"))

(event EventBeginPlay)

(event Collision|EventActorBeginOverlap
  (params (OtherActor :type Actor%20Object%20Reference)))

(event Game|Damage|EventAnyDamage
  (params (Damage :type Float%20%28single-precision%29) (DamageType :type Damage%20Type%20Object%20Reference) (InstigatedBy :type Controller%20Object%20Reference) (DamageCauser :type Actor%20Object%20Reference))
  (bind _cube (Variables|Default|GetCube))
  (Variables|Default|Sethealth (- (Variables|Default|Gethealth) Damage))
  (Utilities|IsValid _cube
    (:Is%20Valid
      (if (<= (Variables|Default|Gethealth) 0.0)
        (Components|DestroyComponent _cube)))))

(fn ConstructionScript)