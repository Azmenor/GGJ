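; BP_Missile is a trap actor that reveals and launches one of three missile components when a BP_Player overlaps it.
; BeginPlay gathers the components into an array, and the overlap unhides a randomly picked one and plays the MissileMove timeline.
; Each timeline update adds the track value to relative X, re-rolling the random index, so the moving missile can differ from the revealed one.
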(event EventBeginPlay
  (Variables|Default|SetArray (Utilities|Array|MakeArray (Variables|Default|GetMissile) (Variables|Default|GetMissile1) (Variables|Default|GetMissile2))))

(event Collision|EventActorBeginOverlap
  (params (OtherActor :type Actor%20Object%20Reference))
  (bind _returnvalue (Math|Random|RandomIntegerinRange 0 2))
  (bind _array (Variables|Default|GetArray))
  (bind _output (Utilities|Array|Get(acopy) _array _returnvalue))
  (bind _relativelocation (Variables|/Script/Engine.SceneComponent|GetRelativeLocation _output))
  (Utilities|Casting|CastToBP_Player OtherActor)
  (Development|SetHiddeninGame _output false true)
  (bind _newtrack_0 (Timeline|missileMove PlayFromStart)
    (:Update
      (Transformation|SetRelativeLocation _output (Math|Vector|MakeVector (+ (.x _relativelocation) _newtrack_0) (.y _relativelocation) (.z _relativelocation)) false false))))

(event EventTick
  (params (DeltaSeconds :type Float%20%28single-precision%29)))

(fn ConstructionScript)