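; BP_Engrenage is a gear actor that spins its static mesh and passes the motion to a linked gear.
; A timeline drives the mesh's relative pitch, signed by the direction, and can start at BeginPlay through a flag.
; Rotate calls the linked gear with the direction negated, so chained gears alternate their spin.
; StopRotate propagates along the same link and stops each timeline.
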(event Custom|Rotate
  (params (Angle%20Direction :type Integer))
  (bind _output_get (Variables|Default|SetAngle%20Direction Angle%20Direction))
  (bind _bp_engrenage (Variables|Default|GetBP_Engrenage)
    (:then
      (CallFunction|Rotate _bp_engrenage (* _output_get -1))
      (bind _rotation (Timeline|Rotation Play)
        (:Update
          (Transformation|SetRelativeRotation (Variables|Default|GetStaticMesh) (Math|Rotator|MakeRotator 0.0 (* (Variables|Default|GetAngle%20Direction) _rotation) 0.0) false false))))
    (:else
      (Timeline|Rotation Play))))

(event Custom|StopRotate
  (bind _bp_engrenage (Variables|Default|GetBP_Engrenage)
    (:then
      (CallFunction|StopRotate _bp_engrenage)
      (bind _rotation (Timeline|Rotation Stop)
        (:Update
          (Transformation|SetRelativeRotation (Variables|Default|GetStaticMesh) (Math|Rotator|MakeRotator 0.0 (* (Variables|Default|GetAngle%20Direction) _rotation) 0.0) false false))))
    (:else
      (Timeline|Rotation Stop))))

(event EventBeginPlay
  (if (Variables|Default|GetShouldStarRotating)
    (CallFunction|Rotate (Variables|Default|GetAngle%20Direction))))

(fn ConstructionScript)