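; Puzzle piston actor whose cylinder moves along Z, acting as either a lethal hazard or a player-triggered mover depending on the Kill flag.
; In Kill mode, a looping timer flip-flops a timeline to cycle the cylinder, and player overlap with the Death volume calls Death on the player.
; Otherwise, the Box trigger plays the Up timeline and the Death volume reverses it, using a reduced offset from the position cached at construction.
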(event OnComponentBeginOverlap(Box)
  (params (OverlappedComponent :type Primitive%20Component%20Object%20Reference) (OtherActor :type Actor%20Object%20Reference) (OtherComp :type Primitive%20Component%20Object%20Reference) (OtherBodyIndex :type Integer) (bFromSweep :type Boolean) (SweepResult :type Hit%20Result%20Structure%20%28by%20ref%29))
  (bind _location (Variables|Default|Getlocation))
  (if (not (Variables|Default|Getkill))
    (Utilities|Casting|CastToBP_Player OtherActor)
    (bind _move (Timeline|Up PlayFromStart)
      (:Update
        (Transformation|SetRelativeLocation (Variables|Default|GetCylinder) (Math|Vector|MakeVector (.x _location) (.y _location) (+ (.z _location) (* _move (- (Variables|Default|Getoffset) 5e+02)))) false false)))))

(event OnComponentBeginOverlap(Death)
  (params (OverlappedComponent :type Primitive%20Component%20Object%20Reference) (OtherActor :type Actor%20Object%20Reference) (OtherComp :type Primitive%20Component%20Object%20Reference) (OtherBodyIndex :type Integer) (bFromSweep :type Boolean) (SweepResult :type Hit%20Result%20Structure%20%28by%20ref%29))
  (bind _location (Variables|Default|Getlocation))
  (if (Variables|Default|Getkill)
    (bind _asbp_player (Utilities|Casting|CastToBP_Player OtherActor))
    (Default|Death _asbp_player)
    (else
      (Utilities|Casting|CastToBP_Player OtherActor)
      (Development|PrintString "Hello")
      (bind _move (Timeline|Up Reverse)
        (:Update
          (Transformation|SetRelativeLocation (Variables|Default|GetCylinder) (Math|Vector|MakeVector (.x _location) (.y _location) (+ (.z _location) (* _move (- (Variables|Default|Getoffset) 5e+02)))) false false))))))

(event Custom|Deplacement
  (bind _location (Variables|Default|Getlocation))
  (Utilities|FlowControl|FlipFlop
    (:A
      (bind _aller_retour (Timeline|Timeline_0 PlayFromStart)
        (:Update
          (Transformation|SetRelativeLocation (Variables|Default|GetCylinder) (Math|Vector|MakeVector (.x _location) (.y _location) (+ (.z _location) (* (Variables|Default|Getoffset) _aller_retour))) false false))))
    (:B
      (Timeline|Timeline_0 ReverseFromEnd))))

(event EventBeginPlay
  (if (Variables|Default|Getkill)
    (Utilities|Time|SetTimerbyEvent (delegate Custom|Deplacement) 2.0 true)))

(fn ConstructionScript
  (Variables|Default|Setlocation (Variables|/Script/Engine.SceneComponent|GetRelativeLocation (Variables|Default|GetCylinder))))