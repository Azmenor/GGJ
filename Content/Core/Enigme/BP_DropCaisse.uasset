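; BP_DropCaisse is a puzzle crate (caisse) that drops or launches through physics.
; Interact turns on physics simulation for the crate, while Launch also applies an upward impulse.
; A Box trigger activates the NSSpark effect when a BP_Rouage actor begins overlapping it and deactivates it when that overlap ends.
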(event OnComponentBeginOverlap(Box)
  (params (OverlappedComponent :type Primitive%20Component%20Object%20Reference) (OtherActor :type Actor%20Object%20Reference) (OtherComp :type Primitive%20Component%20Object%20Reference) (OtherBodyIndex :type Integer) (bFromSweep :type Boolean) (SweepResult :type Hit%20Result%20Structure%20%28by%20ref%29))
  (Utilities|Casting|CastToBP_Rouage OtherActor)
  (Components|Activation|Activate (Variables|Default|GetNS_Spark) false))

(event OnComponentEndOverlap(Box)
  (params (OverlappedComponent :type Primitive%20Component%20Object%20Reference) (OtherActor :type Actor%20Object%20Reference) (OtherComp :type Primitive%20Component%20Object%20Reference) (OtherBodyIndex :type Integer))
  (Utilities|Casting|CastToBP_Rouage OtherActor)
  (Components|Activation|Deactivate (Variables|Default|GetNS_Spark)))

(event Custom|Launch
  (bind _caisse (Variables|Default|GetCaisse))
  (Physics|SetSimulatePhysics _caisse true)
  (Physics|AddImpulse _caisse "0.000000,0.000000,4000.000000" "None" false))

(event Collision|EventActorBeginOverlap
  (params (OtherActor :type Actor%20Object%20Reference)))

(event EventTick
  (params (DeltaSeconds :type Float%20%28single-precision%29)))

(event EventInteract
  (Physics|SetSimulatePhysics (Variables|Default|GetCaisse) true))

(fn ConstructionScript)