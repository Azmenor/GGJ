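; BP_Pince is a puzzle pincer (Enigme folder) whose Cube slides back and forth along its relative Y axis from BeginPlay.
; The construction script caches the Cube's starting relative location, and the Aller timeline scales Offset to displace it from there.
; A FlipFlop re-triggered on timeline Finished alternates forward and reverse playback, producing an endless ping-pong without Tick.
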(event Custom|Deplacement
  (bind _location (Variables|Default|Getlocation))
  (Utilities|FlowControl|FlipFlop :!label _label
    (:A
      (bind _aller_retour (Timeline|aller PlayFromStart)
        (:Update
          (Transformation|SetRelativeLocation (Variables|Default|GetCube) (Math|Vector|MakeVector (.x _location) (+ (.y _location) (* (Variables|Default|Getoffset) _aller_retour)) (.z _location)) false false))
        (:Finished
          (goto _label))))
    (:B
      (Timeline|aller ReverseFromEnd))))

(event EventBeginPlay
  (CallFunction|Deplacement))

(event Collision|EventActorBeginOverlap
  (params (OtherActor :type Actor%20Object%20Reference)))

(event EventTick
  (params (DeltaSeconds :type Float%20%28single-precision%29)))

(fn ConstructionScript
  (Variables|Default|Setlocation (Variables|/Script/Engine.SceneComponent|GetRelativeLocation (Variables|Default|GetCube))))